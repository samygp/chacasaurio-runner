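; GM_Normal is the child game mode for normal, finite levels in the runner, extending its parent's events with level progress and win/lose screens.
; Each floor passed recalculates progress against the FloorMgr floor list, triggering Win at 100% with a final score widget and next-level menu.
; LoadUI adds a progress widget to the Marcador HUD, and GameOver shows its own menu.
; TimerDuration starts from the level config limit, with a countdown function override.
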(event `self.ReceiveBeginPlay`
  ;[1 1 1] BeginPlay
  (`parent.ReceiveBeginPlay`)
  (set `self.TimerDuration` (`/Game/NarutoRunner/Bluprins/Utils/NivelConfig.LimiteTiempo` (`self.NivelConfig`))))

(event `self.ReceiveTick`
  (params (DeltaSeconds :type "Float (single-precision)"))
  ;[1 1 1] On Tick
  (`parent.ReceiveTick` DeltaSeconds))

(event `self.ColisionObstaculo`
  (params (Obstaculo :type "/Game/NarutoRunner/Bluprins/Obstaculos/Obstaculo Object Reference"))
  ;[1 1 1] Colision Obstaculo
  (`parent.ColisionObstaculo` Obstaculo))

(event `self.EvtSpawnPiso`
  ;[1 1 1] Event Spawn Piso
  (`parent.EvtSpawnPiso`))

(event `self.PisoRecorrido`
  ;[1 1 1] Event Piso Recorrido
  (`parent.PisoRecorrido`)
  (bind _resultado (`self.CalcularPorcentajeRecorrido`))
  (if (>= _resultado 1.0)
    (`self.Win`)))

(event `self.Game Over`
  ;[1 1 1] Game Over
  (`parent.Game Over`)
  (`self.MostrarMenu` "/Game/NarutoRunner/Bluprins/UI/Menus/UI_Menu_GameOverNormal.UI_Menu_GameOverNormal_C"))

(event `self.Win`
  ;[1 1 1] Win
  (`parent.Win`)
  (`self.FinalScore`)
  (`self.MostrarMenu` "/Game/NarutoRunner/Bluprins/UI/Menus/UI_WinSiguienteNivel.UI_WinSiguienteNivel_C"))

(fn `CalcularPorcentajeRecorrido`
  (returns (Resultado :type "Float (double-precision)"))
  (bind _output_get (set `self.PorcentajeRecorrido` (/ (`KismetMathLibrary.Conv_IntToDouble` (`self.PisosRecorridos`)) (`KismetMathLibrary.Conv_IntToDouble` (+ (`KismetArrayLibrary.Array_LastIndex` (`/Game/NarutoRunner/Bluprins/Utils/FloorManager.ListaPisos` (`self.FloorMgr`))) 1)))))
  (return _output_get))

(fn `FinalScore`
  (bind _marcador (`self.Marcador`))
  (bind _returnvalue (`|CreateWidget` "/Game/NarutoRunner/Bluprins/UI/Menus/MenuWidgets/Menu_comp_FinalScoreNormal.Menu_comp_FinalScoreNormal_C"))
  (`/Game/NarutoRunner/Bluprins/UI/HUD/HUD_Marcador.ApendizarWidget` _marcador (`/Game/NarutoRunner/Bluprins/UI/HUD/HUD_Marcador.CanvasCentro` _marcador) _returnvalue 0.0 0.0))

(fn `LoadUI`
  (bind _marcador (`self.Marcador`))
  (`parent.LoadUI`)
  (bind _returnvalue (`|CreateWidget` "/Game/NarutoRunner/Bluprins/UI/HUD/HUD_comp_Progreso_Nivel.HUD_comp_Progreso_Nivel_C"))
  (`/Game/NarutoRunner/Bluprins/UI/HUD/HUD_Marcador.ApendizarWidget` _marcador (`/Game/NarutoRunner/Bluprins/UI/HUD/HUD_Marcador.CanvasProgreso` _marcador) _returnvalue 0.0 0.0))

(fn `UpdateTimerDuration`
  (params (`Delta seconds` :type "Float (double-precision)"))
  (set `self.TimerDuration` (- (`self.TimerDuration`) (`KismetMathLibrary.MakeTimespan` 0 0 0 0 (`KismetMathLibrary.FTrunc` (* 1000 `Delta seconds`))))))

(fn `UserConstructionScript`
  (`parent.UserConstructionScript`))