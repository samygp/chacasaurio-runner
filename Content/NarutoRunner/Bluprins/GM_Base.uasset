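; Base game mode for an endless runner that manages level startup, score, timer, pause and win/game-over.
; BeginPlay polls for the level's NivelConfig actor, then spawns the FloorManager, HUD and initial floors before a countdown enables movement.
; Consecutive floors raise the score multiplier, while obstacle hits reset it.
; While the timer runs, Tick shifts the world origin when the next floor spawn passes a Y threshold.
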(event `PisoRecorrido`
  ;[1 1 1] On PisoRecorrido
  (`self.Actualizar Puntos` (`/Game/NarutoRunner/Bluprins/Utils/NivelConfig.PuntosPorPiso` (`self.NivelConfig`)))
  (`/Engine/EditorBlueprintResources/StandardMacros.IncrementInt` (`self.PisosRecorridos`)
    (:`  `
      (`/Engine/EditorBlueprintResources/StandardMacros.IncrementInt` (`self.PisosConsecutivos`)
        (:`  `
          (`self.Actualizar Multiplicador Puntos`))))))

(event `EvtSpawnPiso`
  ;[1 1 1] Spawn Piso Evt
  (`/Game/NarutoRunner/Bluprins/Utils/FloorManager.SiguientePiso` (`self.FloorMgr`)))

(event `ColisionObstaculo`
  (params (Obstaculo :type "/Game/NarutoRunner/Bluprins/Obstaculos/Obstaculo Object Reference"))
  ;[1 1 1] Colisión Obstáculo
  (`self.Actualizar Puntos` (`/Game/NarutoRunner/Bluprins/Obstaculos/Obstaculo.PuntosColision` Obstaculo))
  (set `self.PisosConsecutivos` 0)
  (set `/Game/NarutoRunner/Bluprins/ChacasaurioPlayer.MultiplicadorPuntos` 1 (`self.Jugador`))
  (set `/Game/NarutoRunner/Bluprins/UI/HUD/HUD_Marcador.MultiplicadorTexto` "" (`self.Marcador`))
  (`/Engine/EditorBlueprintResources/StandardMacros.IncrementInt` (`self.Accidentes`)))

(event `self.ReceiveBeginPlay`
  ;[1 1 1] BeginPlay
  (set `PlayerController.bShowMouseCursor` false (`GameplayStatics.GetPlayerController` 0))
  (bind _returnvalue (`self.GetConfig` :!label _label))
  (if _returnvalue
    (`self.Init`)
    (`self.LoadUI`)
    (`self.SpawnPisosIniciales`)
    (`self.Start`)
    (else
      (`KismetSystemLibrary.Delay` 0.3)
      (goto _label))))

(event `Start`
  ;[1 1 1] BeginPlay
  (`/Game/NarutoRunner/Bluprins/Utils/ChacaMacroLibrary.LevelCountdown` (`self.Marcador`))
  (set `/Game/NarutoRunner/Bluprins/ChacasaurioPlayer.CanMove` true (`self.Jugador`))
  (set `self.TimerRunning` true))

(event `Game Over`
  ;[1 1 1] Win / Game Over
  (set `self.TimerRunning` false :!label _label_2)
  (set `/Game/NarutoRunner/Bluprins/ChacasaurioPlayer.CanMove` false (`self.Jugador`))
  (`KismetSystemLibrary.Delay` 1.0))

(event `self.ReceiveTick`
  (params (DeltaSeconds :type "Float (single-precision)"))
  ;[1 1 1] Validar shift origin
  (bind _result (`/Game/NarutoRunner/Bluprins/Utils/ChacaFunctionLibrary.GetDurationString` (`self.TimerDuration`)))
  (set `/Game/NarutoRunner/Bluprins/UI/HUD/HUD_Marcador.TimerTexto` _result (`self.Marcador`))
  (if (`self.TimerRunning`)
    (`self.UpdateTimerDuration` DeltaSeconds)
    (if (not (`self.WorldIsShifting`))
      (`self.Shift Origin`))))

(event `Win`
  ;[1 1 1] Win / Game Over
  (`Widget.SetVisibility` (`self.Marcador`) "Hidden")
  (goto _label_2))

(event `Pausa`
  ;[1 1 1] Pausa y des-pausa
  (`GameplayStatics.SetGamePaused` true)
  (bind _returnvalue (`|CreateWidget` "/Game/NarutoRunner/Bluprins/UI/Menus/UI_Menu_Pausa.UI_Menu_Pausa_C"))
  (`UserWidget.AddToViewport` _returnvalue 0))

(event `Des-pausa`
  ;[1 1 1] Pausa y des-pausa
  (bind _foundwidgets (`WidgetBlueprintLibrary.GetAllWidgetsOfClass` "/Game/NarutoRunner/Bluprins/UI/Menus/UI_Menu_Pausa.UI_Menu_Pausa_C"))
  (for _array_element _foundwidgets
    (`Widget.RemoveFromParent` _array_element)
    (`GameplayStatics.SetGamePaused` false)))

(fn `Actualizar Multiplicador Puntos`
  (bind _jugador (`self.Jugador`))
  (if (== 0 (mod (`self.PisosConsecutivos`) (* (`/Game/NarutoRunner/Bluprins/ChacasaurioPlayer.MultiplicadorPuntos` (`self.Jugador`)) 20)))
    (`/Game/NarutoRunner/Bluprins/ChacasaurioPlayer.IncrementarMultiplicador` _jugador)
    (set `/Game/NarutoRunner/Bluprins/UI/HUD/HUD_Marcador.MultiplicadorTexto` (`KismetStringLibrary.Concat_StrStr` "x " (`KismetStringLibrary.Conv_IntToString` (`/Game/NarutoRunner/Bluprins/ChacasaurioPlayer.MultiplicadorPuntos` _jugador))) (`self.Marcador`))))

(fn `Actualizar Puntos`
  (params (DeltaPuntos :type Integer :default 10))
  (bind _resultado (`self.calcularDeltaPuntos` DeltaPuntos))
  (if (< _resultado 0)
    (`/Game/NarutoRunner/Bluprins/UI/HUD/HUD_Marcador.PuntosMenos` (`self.Marcador`) _resultado)
    (return)))

(fn `calcularDeltaPuntos`
  (params (DeltaPuntos :type Integer))
  (returns (Resultado :type Integer))
  (locals (Result :type Integer :default 0))
  (bind _output_get (set `local.Result` (`KismetMathLibrary.Max` (* (`/Game/NarutoRunner/Bluprins/ChacasaurioPlayer.MultiplicadorPuntos` (`self.Jugador`)) DeltaPuntos) DeltaPuntos)))
  (set `self.Puntos` (`KismetMathLibrary.Clamp` (+ _output_get (`self.Puntos`)) 0 9999999))
  (return (`local.Result`)))

(fn `GetConfig`
  (returns (ReturnValue :type Boolean))
  (bind _outactors (`GameplayStatics.GetAllActorsOfClass` "/Game/NarutoRunner/Bluprins/Utils/NivelConfig.NivelConfig_C"))
  (for _array_element _outactors
    (set `self.NivelConfig` _array_element))
  (return (`KismetSystemLibrary.IsValid` (`self.NivelConfig`))))

(fn `Init`
  (bind _aschacasaurio_player (cast `/Game/NarutoRunner/Bluprins/ChacasaurioPlayer` (`GameplayStatics.GetPlayerCharacter` 0)))
  (set `self.Jugador` _aschacasaurio_player)
  (bind _returnvalue (`|SpawnActorFromClass` "/Game/NarutoRunner/Bluprins/Utils/FloorManager.FloorManager_C" (`KismetMathLibrary.MakeTransform` (0.0 0.0 0.0)) "Undefined" "OverrideRootScale" null (`self.NivelConfig`) (`self.Jugador`) self null))
  (set `self.FloorMgr` _returnvalue))

(fn `LoadUI`
  (bind _marcador (`self.Marcador`))
  (bind _aschacasaurio_player (cast `/Game/NarutoRunner/Bluprins/ChacasaurioPlayer` (`GameplayStatics.GetPlayerCharacter` 0)))
  (bind _returnvalue (`|CreateWidget` "/Game/NarutoRunner/Bluprins/UI/HUD/HUD_Marcador.HUD_Marcador_C"))
  (bind _output_get (set `self.Marcador` _returnvalue))
  (bind _output_get_2 (set `/Game/NarutoRunner/Bluprins/ChacasaurioPlayer.Marcador` _output_get _aschacasaurio_player))
  (`UserWidget.AddToViewport` _output_get_2 0)
  (bind _output_get_3 (set `self.Vidas` (`/Game/NarutoRunner/Bluprins/Utils/NivelConfig.VidasIniciales` (`self.NivelConfig`))))
  (`/Game/NarutoRunner/Bluprins/UI/HUD/HUD_Marcador.AgregarVidas` (`self.Marcador`) _output_get_3)
  (if (`/Game/NarutoRunner/Bluprins/Utils/NivelConfig.MostrarHUD` (`self.NivelConfig`))
    (`Widget.SetVisibility` _marcador "Visible")
    (else
      (`Widget.SetVisibility` _marcador "Hidden"))))

(fn `MostrarMenu`
  (params (WidgetClass :type "UserWidget Class Reference"))
  (bind _returnvalue (`|CreateWidget` WidgetClass))
  (`UserWidget.AddToViewport` _returnvalue 0))

(fn `Shift Origin`
  (locals (ReferencePosition :type "Vector Structure"))
  (bind _nuevosuelospawn_location (`KismetMathLibrary.BreakTransform` (`/Game/NarutoRunner/Bluprins/Utils/FloorManager.NuevoSueloSpawn` (`self.FloorMgr`))))
  (bind _output_get (set `local.ReferencePosition` (`KismetMathLibrary.Conv_IntVectorToVector` (`KismetMathLibrary.FTruncVector` _nuevosuelospawn_location))))
  (if (> (`KismetMathLibrary.Abs` (.y _output_get)) (`/Game/NarutoRunner/Bluprins/Utils/NivelConfig.WorldShiftThreshold` (`self.NivelConfig`)))
    (set `self.WorldIsShifting` true)
    (`GameplayStatics.SetWorldOriginLocation` (`KismetMathLibrary.FTruncVector` (+ (`local.ReferencePosition`) (`KismetMathLibrary.Conv_IntVectorToVector` (`GameplayStatics.GetWorldOriginLocation`)))))
    (set `/Game/NarutoRunner/Bluprins/Utils/FloorManager.NuevoSueloSpawn` (`KismetMathLibrary.MakeTransform` (0.0 0.0 0.0)) (`self.FloorMgr`))
    (set `self.WorldIsShifting` false)))

(fn `SpawnPisosIniciales`
  (for _ (range (+ (- (`/Game/NarutoRunner/Bluprins/Utils/NivelConfig.LimitePisos` (`self.NivelConfig`)) 5) 1))
    (`/Game/NarutoRunner/Bluprins/Utils/FloorManager.SiguientePiso` (`self.FloorMgr`))))

(fn `UpdateTimerDuration`
  (params (`Delta seconds` :type "Float (double-precision)")))

(fn `UserConstructionScript`)