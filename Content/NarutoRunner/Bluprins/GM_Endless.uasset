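; Endless-mode game mode for the runner, a child Blueprint that passes floor spawning, floor progress and obstacle collision events to its parent.
; Game over runs the parent logic, then opens the endless game-over menu, while FinalScore appends a score widget to the center canvas of Marcador.
; The timer counts up by adding delta seconds as whole milliseconds.
; The completion-percentage function is empty, with its floor-target calculation left unused.
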(event `self.ReceiveBeginPlay`
  ;[1 1 1] BeginPlay
  (`parent.ReceiveBeginPlay`))

(event `self.ReceiveTick`
  (params (DeltaSeconds :type "Float (single-precision)"))
  ;[1 1 1] On Tick
  (`parent.ReceiveTick` DeltaSeconds))

(event `self.EvtSpawnPiso`
  ;[1 1 1] Event Spawn Piso
  (`parent.EvtSpawnPiso`))

(event `self.PisoRecorrido`
  ;[1 1 1] Event Piso Recorrido
  (`parent.PisoRecorrido`))

(event `self.ColisionObstaculo`
  (params (Obstaculo :type "/Game/NarutoRunner/Bluprins/Obstaculos/Obstaculo Object Reference"))
  ;[1 1 1] Colision Obstaculo
  (`parent.ColisionObstaculo` Obstaculo))

(event `self.Game Over`
  ;[1 1 1] Game Over
  (`parent.Game Over`)
  (`self.MostrarMenu` "/Game/NarutoRunner/Bluprins/UI/Menus/UI_Menu_GameOverEndless.UI_Menu_GameOverEndless_C"))

(fn `CalcularPorcentajeRecorrido`
  (returns (Resultado :type "Float (double-precision)")))

(fn `FinalScore`
  (bind _marcador (`self.Marcador`))
  (bind _returnvalue (`|CreateWidget` "/Game/NarutoRunner/Bluprins/UI/Menus/MenuWidgets/Menu_comp_FinalScoreNormal.Menu_comp_FinalScoreNormal_C"))
  (`/Game/NarutoRunner/Bluprins/UI/HUD/HUD_Marcador.ApendizarWidget` _marcador (`/Game/NarutoRunner/Bluprins/UI/HUD/HUD_Marcador.CanvasCentro` _marcador) _returnvalue 0.0 0.0))

(fn `UpdateTimerDuration`
  (params (`Delta seconds` :type "Float (double-precision)"))
  (set `self.TimerDuration` (+ (`self.TimerDuration`) (`KismetMathLibrary.MakeTimespan` 0 0 0 0 (`KismetMathLibrary.FTrunc` (* 1000 `Delta seconds`))))))

(fn `UserConstructionScript`
  (`parent.UserConstructionScript`))